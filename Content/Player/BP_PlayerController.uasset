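; Player controller for a team-based office war game that drives lobby and HUD screens and switches control between team characters.
; It shows the session lobby on begin play, registers confirmation with the game mode, then swaps to the main HUD at round start.
; Primary input fires the possessed character's equipped item, while Interact sphere-traces from the camera to pick up and equip items.
; NextCharacter cycles possession through the Team array.
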(event `self.ReceiveBeginPlay`
  (`self.Create Game Lobby`))

(event `Create Game Lobby`
  (bind _returnvalue (`|CreateWidget` "/Game/Lobby/UI_SessionLobby.UI_SessionLobby_C" self))
  (`UserWidget.AddToViewport` _returnvalue 0))

(event `Register With Game Mode`
  (bind _asbp_office_war_game_mode (cast `/Game/ThirdPersonCPP/Blueprints/BP_OfficeWarGameMode` (`GameplayStatics.GetGameMode`)))
  (`/Game/ThirdPersonCPP/Blueprints/BP_OfficeWarGameMode.LobbyPlayerConfirmed` _asbp_office_war_game_mode self))

(event `Notify Client of Round Start`
  (bind _foundwidgets (`WidgetBlueprintLibrary.GetAllWidgetsOfClass` "/Game/Lobby/UI_SessionLobby.UI_SessionLobby_C" false))
  (for _array_element _foundwidgets
    (`Widget.RemoveFromParent` _array_element))
  (bind _returnvalue (`|CreateWidget` "/Game/Player/UI_MainHUD.UI_MainHUD_C" self))
  (`UserWidget.AddToViewport` _returnvalue 0))

(event `InputAction|Primary`
  (params (Key :type "Key Structure"))
  (bind _returnvalue (`self.K2_GetPawn`))
  (:`Pressed`
    (`/Engine/EditorBlueprintResources/StandardMacros.IsValid` _returnvalue
      (:`Is Valid`
        (bind _asthird_person_character (cast `/Game/ThirdPersonCPP/Blueprints/ThirdPersonCharacter` _returnvalue))
        (bind _inventory (`GameJamCharacter.Inventory` _asthird_person_character))
        (bind _equipped (`GameJamCharacter.Equipped` _asthird_person_character))
        (if (`KismetArrayLibrary.Array_IsValidIndex` _inventory _equipped)
          (bind _output (`|GetArrayItem` _inventory _equipped))
          (`/Engine/EditorBlueprintResources/StandardMacros.IsValid` _output
            (:`Is Valid`
              (`CodeWeapon.PrimaryFunction` _output))))))))

(event `self.NextCharacter`
  (bind _team (`self.Team`))
  (`/Engine/EditorBlueprintResources/StandardMacros.IsValid` (`self.K2_GetPawn`)
    (:`Is Valid`
      (`self.UnPossess`)
      (bind _output_get (set `self.CurrentChar` (mod (+ (`self.CurrentChar`) 1) (`KismetArrayLibrary.Array_Length` _team))))
      (`self.Possess` (`|GetArrayItem` _team _output_get)))))

(event `InputAction|Interact`
  (params (Key :type "Key Structure"))
  (bind _returnvalue (`GameplayStatics.GetPlayerCameraManager` 0))
  (bind _returnvalue_2 (`PlayerCameraManager.GetCameraLocation` _returnvalue))
  (:`Pressed`
    (bind _outhit (`KismetSystemLibrary.SphereTraceSingleForObjects` _returnvalue_2 (+ _returnvalue_2 (* (`self.GetActorForwardVector` _returnvalue) 1000)) 20.0 (`|MakeArray` "ObjectTypeQuery2" :!type "EObjectTypeQuery Enum") true (`self.Team`) "ForOneFrame"))
    (bind _asbp_item (cast `/Game/ThirdPersonCPP/Blueprints/BP_Item` (`.HitActor` (`GameplayStatics.BreakHitResult` _outhit))))
    (bind _asthird_person_character (cast `/Game/ThirdPersonCPP/Blueprints/ThirdPersonCharacter` (`self.K2_GetPawn`)))
    (`/Game/ThirdPersonCPP/Blueprints/ThirdPersonCharacter.Add To Inventory` _asthird_person_character _asbp_item)
    (`/Game/ThirdPersonCPP/Blueprints/ThirdPersonCharacter.Equip Item` _asthird_person_character)))

(fn `UserConstructionScript`)